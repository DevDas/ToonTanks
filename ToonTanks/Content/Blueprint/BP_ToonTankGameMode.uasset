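; BP_ToonTankGameMode is the Toon Tank game mode Blueprint that manages the match's UI and end-of-game camera.
; BeginPlay adds the player HUD, and GameStart shows a start widget fed with the start delay.
; GameOver records the result, shows the win/lose widget, removes the HUD and blends the player's view to the first SpecView actor in the level.
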(event `self.ReceiveBeginPlay`
  (bind _returnvalue (`|CreateWidget` "/Game/UI/WBP_PlayerScreen.WBP_PlayerScreen_C"))
  (`UserWidget.AddToViewport` _returnvalue 0))

(event `self.GameStart`
  (bind _returnvalue (`|CreateWidget` "/Game/UI/WBP_GameStart.WBP_GameStart_C"))
  (`UserWidget.AddToViewport` _returnvalue 0)
  (`/Game/UI/WBP_GameStart.SetStartDelay` _returnvalue (`self.StartDelay`)))

(event `self.GameOver`
  (params (PlayerWon :type Boolean))
  (set `self.Won?` PlayerWon)
  (bind _returnvalue (`|CreateWidget` "/Game/UI/WBP_PlayerWon.WBP_PlayerWon_C"))
  (set `/Game/UI/WBP_PlayerWon.PlayerWon` PlayerWon _returnvalue)
  (`UserWidget.AddToViewport` _returnvalue 0)
  (bind _outactors (`GameplayStatics.GetAllActorsOfClass` "/Game/Blueprint/SpecView.SpecView_C"))
  (`PlayerController.SetViewTargetWithBlend` (`GameplayStatics.GetPlayerController` 0) (`|GetArrayItem` _outactors) 2.0 "VTBlend_Cubic" 0.0 false)
  (`Widget.RemoveFromParent` (stale `self.ReceiveBeginPlay` _returnvalue)))

(fn `UserConstructionScript`)